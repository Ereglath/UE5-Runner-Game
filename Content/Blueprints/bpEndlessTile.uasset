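; Self-chaining track tile for an endless runner-style level that fills itself with random obstacles and coins.
; On BeginPlay it rolls each of six spawn points for a weighted-chance obstacle, falling back to a weighted-chance coin.
; Overlapping the next-tile trigger disables it and spawns another tile at the NextTileMark transform.
; A separate removal trigger destroys the tile, leaving its spawned obstacles and coins untouched.
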(event `self.ReceiveBeginPlay`
  (`self.SpawnObjects`))

(event `self.NEXTileCollision.OnComponentBeginOverlap`
  (params (OverlappedComponent :type "PrimitiveComponent Object Reference") (OtherActor :type "Actor Object Reference") (OtherComp :type "PrimitiveComponent Object Reference") (OtherBodyIndex :type Integer) (bFromSweep :type Boolean) (SweepResult :type "HitResult Structure (by ref)"))
  (`PrimitiveComponent.SetCollisionEnabled` OverlappedComponent "NoCollision")
  (`self.SpawnNextTile`))

(event `self.TileRemoval.OnComponentBeginOverlap`
  (params (OverlappedComponent :type "PrimitiveComponent Object Reference") (OtherActor :type "Actor Object Reference") (OtherComp :type "PrimitiveComponent Object Reference") (OtherBodyIndex :type Integer) (bFromSweep :type Boolean) (SweepResult :type "HitResult Structure (by ref)"))
  (`PrimitiveComponent.SetCollisionEnabled` OverlappedComponent "NoCollision")
  (`self.K2_DestroyActor`))

(fn `GetNextTileSpawnTransform`
  (returns (Loc :type "Transform Structure"))
  (return (`SceneComponent.K2_GetComponentToWorld` (`self.NextTileMark`))))

(fn `SpawnNextTile`
  (`|SpawnActorFromClass` "bpEndlessTile_C" (`self.GetNextTileSpawnTransform`) "AlwaysSpawn" "OverrideRootScale" null null))

(fn `SpawnObjects`
  (for _array_element (`self.SpawnPoints`)
    (bind _returnvalue (`SceneComponent.K2_GetComponentToWorld` _array_element))
    (bind _bspawned (`self.TrySpawnObstacle` _returnvalue))
    (if (not _bspawned)
      (`self.TrySpawnCoin` _returnvalue))))

(fn `TrySpawnCoin`
  (params (Transform :type "Transform Structure"))
  (returns (bSpawned :type Boolean))
  (if (`KismetMathLibrary.RandomBoolWithWeight` (`self.CoinChanse`))
    (`|SpawnActorFromClass` "/Game/Blueprints/bpCoin.bpCoin_C" Transform "Undefined" "OverrideRootScale" null null)
    (return true)
    (else
      (return false))))

(fn `TrySpawnObstacle`
  (params (transform :type "Transform Structure"))
  (returns (bSpawned :type Boolean))
  (if (`KismetMathLibrary.RandomBoolWithWeight` (`self.ObstacleChanse`))
    (`|SpawnActorFromClass` "/Game/Blueprints/bpObstacle.bpObstacle_C" transform "Undefined" "OverrideRootScale" null null)
    (return true)
    (else
      (return false))))

(fn `UserConstructionScript`
  (set `self.SpawnPoints` (`|MakeArray` (`self.Spawn0`) (`self.Spawn1`) (`self.Spawn2`) (`self.Spawn3`) (`self.Spawn4`) (`self.Spawn5`) :!type "SceneComponent Object Reference")))