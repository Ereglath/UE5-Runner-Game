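; HUD Blueprint that shows the main in-game HUD widget and manages a restart menu for the owning player.
; On BeginPlay it creates the WHud widget and adds it to the viewport.
; OpenRestartMenu creates the restart menu, binds to its OnSelected event and switches to UI-only input with a visible cursor.
; When a selection fires, it removes the menu and restores game-only input with the cursor hidden.
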(event `self.ReceiveBeginPlay`
  (bind _returnvalue (`|CreateWidget` "/Game/Blueprints/wHud.wHud_C" (`self.PlayerOwner`)))
  (bind _output_get (set `self.wHud` _returnvalue))
  (`UserWidget.AddToViewport` _output_get 0))

(event `OpenRestartMenu`
  (bind _playerowner (`self.PlayerOwner`))
  (bind _returnvalue (`|CreateWidget` "/Game/Blueprints/wRestartMenu.wRestartMenu_C" (`self.PlayerOwner`)))
  (bind _output_get (set `self.wRestart` _returnvalue))
  (add `/Game/Blueprints/wRestartMenu.OnSelected` _output_get (delegate `OnRestartSelected`))
  (`UserWidget.AddToViewport` (`self.wRestart`) 0)
  (`WidgetBlueprintLibrary.SetInputMode_UIOnlyEx` _playerowner null)
  (set `PlayerController.bShowMouseCursor` true _playerowner))

(event `OnRestartSelected`
  (bind _playerowner (`self.PlayerOwner`))
  (`Widget.RemoveFromParent` (`self.wRestart`))
  (set `self.wRestart` null)
  (`WidgetBlueprintLibrary.SetInputMode_GameOnly` _playerowner)
  (set `PlayerController.bShowMouseCursor` false _playerowner))

(fn `UserConstructionScript`)